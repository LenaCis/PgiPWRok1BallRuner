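; BP_hammer is a swinging hammer hazard that damages the player pawn on contact.
; Tick runs through a 1.5-second Delay to repeatedly restart the HammerFall timeline, whose TLUderzenie track drives the world roll of the handle component Rączka.
; A Box overlap applies damage when the other actor is player pawn 0, and otherwise prints a debug string.
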(event OnComponentBeginOverlap(Box)
  (params (OverlappedComponent :type Primitive%20Component%20Object%20Reference) (OtherActor :type Actor%20Object%20Reference) (OtherComp :type Primitive%20Component%20Object%20Reference) (OtherBodyIndex :type Integer) (bFromSweep :type Boolean) (SweepResult :type Hit%20Result%20Structure%20%28by%20ref%29))
  (if (== OtherActor (Game|Player|GetPlayerPawn 0))
    (Game|Damage|ApplyDamage (Game|Player|GetPlayerPawn 0) 1.0 0 0)
    (else
      (Development|PrintString "nie zderzył się"))))

(event EventTick
  (params (DeltaSeconds :type Float%20%28single-precision%29))
  (Utilities|FlowControl|Delay 1.5)
  (bind _tl_uderzenie (Timeline|hammer%20fall PlayFromStart)
    (:Update
      (Transformation|SetWorldRotation (Variables|Default|Getrączka) (Math|Rotator|MakeRotator _tl_uderzenie 0.0 0.0) false false))))

(fn ConstructionScript)