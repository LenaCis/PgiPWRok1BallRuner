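; End-of-level trigger that advances the player to the next level once every crystal has been collected.
; When the player pawn overlaps its box, it checks for remaining BP_Crystal_01 actors and prints a Polish warning if any are left.
; Otherwise it finds the current level's name in ArrayLevel and opens the following entry, or quits the game on the last level.
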(event OnComponentBeginOverlap(Box)
  (params (OverlappedComponent :type Primitive%20Component%20Object%20Reference) (OtherActor :type Actor%20Object%20Reference) (OtherComp :type Primitive%20Component%20Object%20Reference) (OtherBodyIndex :type Integer) (bFromSweep :type Boolean) (SweepResult :type Hit%20Result%20Structure%20%28by%20ref%29))
  (if (== OtherActor (Game|Player|GetPlayerPawn 0))
    (bind _returnvalue (CallFunction|CheckAnyCrystals))
    (if _returnvalue
      (Development|PrintString "Nie zebrales wszystkich krysztalow")
      (else
        (CallFunction|CompleteLvl)))))

(fn ConstructionScript)

(fn CheckAnyCrystals
  (bind _outactors (Actor|GetAllActorsOfClass "/Game/BluePrints/BP_Crystal_01.BP_Crystal_01_C"))
  (return (> (Utilities|Array|Length _outactors) 0)))

(fn CurrentLevelIndex
  (bind _returnvalue (Game|GetCurrentLevelName true))
  (return (Utilities|Array|FindItem (Variables|Default|GetArray%20Level) (Utilities|String|StringToName _returnvalue))))

(fn CompleteLvl
  (if (CallFunction|IsLastLvl)
    (Game|QuitGame 0 "Quit" false)
    (else
      (Development|PrintString "Brawo -  następny lvl")
      (Game|OpenLevel(byName) (CallFunction|LoadNextLvl)))))

(fn IsLastLvl
  (return (== (CallFunction|CurrentLevelIndex) (Utilities|Array|LastIndex (Variables|Default|GetArray%20Level)))))

(fn LoadNextLvl
  (return (Utilities|Array|Get(acopy) (Variables|Default|GetArray%20Level) (+ (CallFunction|CurrentLevelIndex) 1))))