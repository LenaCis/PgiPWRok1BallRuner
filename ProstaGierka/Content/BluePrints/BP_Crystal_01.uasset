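; BP_Crystal_01 is a crystal actor that flies into the player and vanishes when the player pawn overlaps its sphere.
; One timeline drives the effect with separate curves for location, scale and point light intensity (Miganie).
; Position and scale lerp from their current values every update, so the crystal homes on the moving pawn while shrinking.
; The actor destroys itself when the timeline finishes, without notifying other objects.
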(event OnComponentBeginOverlap(Sphere)
  (params (OverlappedComponent :type Primitive%20Component%20Object%20Reference) (OtherActor :type Actor%20Object%20Reference) (OtherComp :type Primitive%20Component%20Object%20Reference) (OtherBodyIndex :type Integer) (bFromSweep :type Boolean) (SweepResult :type Hit%20Result%20Structure%20%28by%20ref%29))
  (if (== OtherActor (Game|Player|GetPlayerPawn 0))
    (bind (_direction _crystal_location _crystal_scale _miganie) (Timeline|Timeline_1 Play)
      (:Update
        (Transformation|SetActorLocation (Math|Vector|Lerp(Vector) (Transformation|GetActorLocation) (Transformation|GetActorLocation (Game|Player|GetPlayerPawn 0)) _crystal_location) false false)
        (Transformation|SetActorScale3D (Math|Vector|Lerp(Vector) (Transformation|GetActorScale3D) "0, 0, 0" _crystal_scale))
        (Rendering|Components|Light|SetIntensity (Variables|Default|GetPointLight) (Math|Float|Lerp 5e+04 0.0 _miganie)))
      (:Finished
        (Actor|DestroyActor)))))

(fn ConstructionScript)