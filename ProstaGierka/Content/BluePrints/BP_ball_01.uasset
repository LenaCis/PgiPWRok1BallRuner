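; BP_ball_01 is a physics-driven ball, rolled by torque on its Sphere from movement input.
; Both movement axes share one torque call, applying the scaled value to X and Y alike.
; A hit from BP_Pocisk turns off the sphere's collision.
; The screen fades from black on BeginPlay; the first damage received fades it out and reloads the current level.
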(event OnComponentHit(Sphere)
  (params (HitComponent :type Primitive%20Component%20Object%20Reference) (OtherActor :type Actor%20Object%20Reference) (OtherComp :type Primitive%20Component%20Object%20Reference) (NormalImpulse :type Vector :default "0, 0, 0") (Hit :type Hit%20Result%20Structure%20%28by%20ref%29))
  (if (== OtherActor "/Game/BluePrints/BP_Pocisk.BP_Pocisk")
    (Collision|SetCollisionEnabled (Variables|Default|GetSphere) "NoCollision")))

(event Game|Damage|EventAnyDamage
  (params (Damage :type Float%20%28single-precision%29) (DamageType :type Damage%20Type%20Object%20Reference) (InstigatedBy :type Controller%20Object%20Reference) (DamageCauser :type Actor%20Object%20Reference))
  (Utilities|FlowControl|DoOnce false
    (:Completed
      (CameraFades|StartCameraFade :self (Game|GetPlayerCameraManager 0) :ToAlpha 1.0 :Duration 2.0 :bHoldWhenFinished true)
      (Utilities|FlowControl|Delay 2.0)
      (bind _returnvalue (Game|GetCurrentLevelName true))
      (Game|OpenLevel(byName) (Utilities|String|StringToName _returnvalue)))))

(event EventBeginPlay
  (CameraFades|StartCameraFade :self (Game|GetPlayerCameraManager 0) :FromAlpha 1.0 :Duration 2.0 :bHoldWhenFinished true))

(event Input|AxisEvents|InputAxismove_forward_back
  (params (AxisValue :type Float%20%28single-precision%29))
  (bind _multiply (Variables|Default|GetMultiply))
  (Class|PrimitiveComponent|AddTorqueinRadians (Variables|Default|GetSphere) (Math|Vector|MakeVector (* (stale Input|AxisEvents|InputAxismove_left_right AxisValue) _multiply) (* AxisValue _multiply) 0.0) "None" true))

(event Input|AxisEvents|InputAxismove_left_right
  (params (AxisValue :type Float%20%28single-precision%29))
  (bind _multiply (Variables|Default|GetMultiply))
  (Class|PrimitiveComponent|AddTorqueinRadians (Variables|Default|GetSphere) (Math|Vector|MakeVector (* AxisValue _multiply) (* (stale Input|AxisEvents|InputAxismove_forward_back AxisValue) _multiply) 0.0) "None" true))

(fn ConstructionScript)